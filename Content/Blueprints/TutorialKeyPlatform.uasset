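; Tutorial variant of a key platform that prompts the player to take the Golden Skull in the maze game.
; Extends parent enter, leave and interact events, writing to the MazeGameMode's PlayerUI message.
; Entering shows a prompt with the bound interact key's display name while the skull is untaken.
; Leaving, or interacting once it is taken, clears the message.
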(event EventOnEnter
  (params (OtherActor :type Object%20Object%20Reference))
  ;[1 1 1] Call to parent
  (|CallParentFunction OtherActor)
  ;[1 1 1] Set Tutorial Message
  (bind _isplayer (CallFunction|IsPlayer OtherActor))
  (if _isplayer
    (if (not (Variables|Default|GetisTaken))
      (bind _asmaze_game_mode (Utilities|Casting|CastToMazeGameMode (Game|GetGameMode)))
      (Variables|/Game/UI/PlayerUI.PlayerUI_C|SetMessage (Variables|/Game/GameSettings/MazeGameMode.MazeGameMode_C|GetPlayerUI _asmaze_game_mode) (Utilities|Text|FormatText "Press '{key}' to take the Golden Skull" (Class|KismetInputLibrary|KeyGetDisplayName (Variables|/Game/GameSettings/MazeGameMode.MazeGameMode_C|GetInteractKey _asmaze_game_mode))))
      (Default|UpdateMessage (Variables|/Game/GameSettings/MazeGameMode.MazeGameMode_C|GetPlayerUI _asmaze_game_mode)))))

(event EventOnLeave
  (params (OtherActor :type Object%20Object%20Reference))
  ;[1 1 1] Call to parent
  (|CallParentFunction OtherActor)
  ;[1 1 1] Clear Tutorial Message
  (bind _isplayer (CallFunction|IsPlayer OtherActor))
  (if _isplayer
    (bind _asmaze_game_mode (Utilities|Casting|CastToMazeGameMode (Game|GetGameMode)))
    (Variables|/Game/UI/PlayerUI.PlayerUI_C|SetMessage (Variables|/Game/GameSettings/MazeGameMode.MazeGameMode_C|GetPlayerUI _asmaze_game_mode) "")
    (Default|UpdateMessage (Variables|/Game/GameSettings/MazeGameMode.MazeGameMode_C|GetPlayerUI _asmaze_game_mode))))

(event EventOnInteract
  ;[1 1 1] Call to parent
  (|CallParentFunction)
  ;[1 1 1] Is Key Taken?
  (if (Variables|Default|GetisTaken)
    ;[1 1 1] Clear Tutorial Message
    (bind _asmaze_game_mode (Utilities|Casting|CastToMazeGameMode (Game|GetGameMode)))
    (Variables|/Game/UI/PlayerUI.PlayerUI_C|SetMessage (Variables|/Game/GameSettings/MazeGameMode.MazeGameMode_C|GetPlayerUI _asmaze_game_mode) "")
    (Default|UpdateMessage (Variables|/Game/GameSettings/MazeGameMode.MazeGameMode_C|GetPlayerUI _asmaze_game_mode))))

(fn ConstructionScript
  (|CallParentFunction))