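; Locked maze door that the player opens by pressing Interact inside its trigger volume, spending one key.
; Trigger overlaps toggle the actor's input for the player, and a successful interact decrements the key count and refreshes the key display through MazeGameMode's UI.
; Opening spawns a collision-free key mesh snapped to the keyhole, plays a sound, and runs a timeline that slides the key and moves the door vertically.
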(event OnComponentBeginOverlap(TriggerVolume)
  (params (OverlappedComponent :type Primitive%20Component%20Object%20Reference) (OtherActor :type Actor%20Object%20Reference) (OtherComp :type Primitive%20Component%20Object%20Reference) (OtherBodyIndex :type Integer) (bFromSweep :type Boolean) (SweepResult :type Hit%20Result%20Structure%20%28by%20ref%29))
  ;[1 1 1] Bind events
  (CallFunction|OnEnter OtherActor))

(event OnComponentEndOverlap(TriggerVolume)
  (params (OverlappedComponent :type Primitive%20Component%20Object%20Reference) (OtherActor :type Actor%20Object%20Reference) (OtherComp :type Primitive%20Component%20Object%20Reference) (OtherBodyIndex :type Integer))
  ;[1 1 1] Bind events
  (CallFunction|OnLeave OtherActor))

(event Custom|OnInteract
  ;[1 1 1] Is Door not Open?
  (if (not (Variables|Default|GetisOpen))
    ;[1 1 1] Player has enough keys?
    (bind _asplayer_character (Utilities|Casting|CastToPlayerCharacter (Game|GetPlayerCharacter 0)))
    (if (> (Variables|/Game/Player/PlayerCharacter.PlayerCharacter_C|GetnumberOfKeys _asplayer_character) 0)
      (Math|Integer|DecrementInt (Variables|/Game/Player/PlayerCharacter.PlayerCharacter_C|GetnumberOfKeys _asplayer_character) :!pinned true ; Take key
        (:%20%20
          (Variables|Default|SetisOpen true :!pinned true) ; Set isOpen
          ;[1 1 1] Update Number Of Keys display
          (bind _asmaze_game_mode (Utilities|Casting|CastToMazeGameMode (Game|GetGameMode)))
          (Default|UpdateNumberOfKeys (Variables|/Game/GameSettings/MazeGameMode.MazeGameMode_C|GetPlayerUI _asmaze_game_mode))
          (CallFunction|OnOpen :!pinned true) ; Send Open Event
        )))))

(event Custom|OnEnter
  (params (OtherActor :type Object%20Object%20Reference))
  ;[1 1 1] Is Player?
  (if (== OtherActor (Game|GetPlayerCharacter 0))
    ;[1 1 1] Enable Input
    (Input|EnableInput (Game|GetPlayerController 0))))

(event Custom|OnLeave
  (params (OtherActor :type Object%20Object%20Reference))
  ;[1 1 1] Is Player?
  (if (== OtherActor (Game|GetPlayerCharacter 0))
    ;[1 1 1] Disable Input
    (Input|DisableInput (Game|GetPlayerController 0))))

(event Custom|OnOpen
  ;[1 1 1] Add Key to Door
  (bind _returnvalue (AddComponent|AddStaticMeshComponent false))
  (bind _output_get (Variables|Default|SetKeyMesh _returnvalue))
  (Collision|SetCollisionEnabled _output_get "NoCollision")
  (Transformation|AttachComponentToComponent _output_get (Variables|Default|GetKeyhole) "None" "SnapToTarget" "SnapToTarget" "SnapToTarget" true)
  ;[1 1 1] Door Opening Sound
  (Audio|PlaySoundatLocation "/Game/Sounds/DoorOpening_SFX.DoorOpening_SFX" (Transformation|GetActorLocation) "0, 0, 0" 1.0 1.0 0.0 0 0 0)
  ;[1 1 1] Door Opening animation
  (bind (_direction _doorposition _keyposition) (Timeline|Door_Open PlayFromStart)
    (:Update
      (Transformation|SetRelativeLocation (Variables|Default|GetKeyMesh) (Math|Vector|MakeVector 0.0 _keyposition 0.0) false false)
      (Transformation|SetRelativeLocation (Variables|Default|GetDoorMesh) (Math|Vector|MakeVector 0.0 0.0 _doorposition) false false))))

(event Input|ActionEvents|InputActionInteract
  (params (Key :type Key%20Structure))
  ;[1 1 1] Bind events
  (:Pressed
    (CallFunction|OnInteract)))

(fn ConstructionScript)