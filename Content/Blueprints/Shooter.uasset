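; Shooter actor that fires arrows along its ArrowSource's forward direction while the player character is in its line of sight.
; Every tick, a sphere trace on the Camera channel runs out to SightRange and checks whether it hits the player.
; A hit triggers ShootArrow, which plays a sound and spawns an Arrow at ArrowSource's transform.
; DoOnce, reset after a ShootInterval delay, limits the fire rate.
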(event Custom|ShootArrow
  ;[1 1 1] Shoot Sound
  (Audio|PlaySoundatLocation "/Game/Sounds/Arrow_SFX.Arrow_SFX" (Transformation|GetActorLocation) "0, 0, 0" 1.0 1.0 0.0 0 0 0)
  ;[1 1 1] Spawn an Arrow
  (Game|SpawnActorfromClass "/Game/Blueprints/Arrow.Arrow_C" (Transformation|GetWorldTransform (Variables|Default|GetArrowSource)) "Undefined" 0 0))

(event EventTick
  (params (DeltaSeconds :type Float%20%28single-precision%29))
  (bind _arrowsource (Variables|Default|GetArrowSource))
  (bind _returnvalue (Transformation|GetWorldLocation _arrowsource))
  ;[1 1 1] Is Player in sight?
  (bind _outhit (Collision|SphereTraceByChannel _returnvalue (+ _returnvalue (* (Math|Vector|GetForwardVector _arrowsource) (Variables|Default|GetSightRange))) (Variables|Default|GetarrowCollisionRadius) "TraceTypeQuery2" false 0 "None" true "(R=1.000000,G=0.000000,B=0.000000,A=1.000000)" "(R=0.000000,G=1.000000,B=0.000000,A=1.000000)" 2.0))
  (if (== (.hitactor _outhit) (Game|GetPlayerCharacter 0))
    ;[1 1 1] Shoot Arrows at interval
    (Utilities|FlowControl|DoOnce false :!label _label
      (:Completed
        (CallFunction|ShootArrow)
        (Utilities|FlowControl|Delay (Variables|Default|GetShootInterval))
        (goto _label Reset)))))

(fn ConstructionScript)