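; A tutorial variant of a maze door that shows on-screen hints when the player approaches it.
; On enter, if the door is closed, it checks the player's key count and sets either a prompt naming the interact key to use the Golden Skull or a hint that something is missing.
; Leaving or opening the door clears the message through the game mode's PlayerUI, after calling the parent door logic.
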(event EventOnEnter
  (params (OtherActor :type Object%20Object%20Reference))
  ;[1 1 1] Call to parent
  (|CallParentFunction OtherActor)
  ;[1 1 1] Set Tutorial Message
  (bind _isplayer (CallFunction|IsPlayer OtherActor))
  (if _isplayer
    (if (not (Variables|Default|GetisOpen))
      (bind _asmaze_game_mode (Utilities|Casting|CastToMazeGameMode (Game|GetGameMode)))
      (bind _asplayer_character (Utilities|Casting|CastToPlayerCharacter (Game|GetPlayerCharacter 0)))
      (if (> (Variables|/Game/Player/PlayerCharacter.PlayerCharacter_C|GetnumberOfKeys _asplayer_character) 0)
        (Variables|/Game/UI/PlayerUI.PlayerUI_C|SetMessage (Variables|/Game/GameSettings/MazeGameMode.MazeGameMode_C|GetPlayerUI _asmaze_game_mode) (Utilities|Text|FormatText "Press '{key}' to use the Golden Skull" (Class|KismetInputLibrary|KeyGetDisplayName (Variables|/Game/GameSettings/MazeGameMode.MazeGameMode_C|GetInteractKey _asmaze_game_mode))))
        (else
          (Variables|/Game/UI/PlayerUI.PlayerUI_C|SetMessage (Variables|/Game/GameSettings/MazeGameMode.MazeGameMode_C|GetPlayerUI _asmaze_game_mode) "Looks like this door is missing something...")))
      (Default|UpdateMessage (Variables|/Game/GameSettings/MazeGameMode.MazeGameMode_C|GetPlayerUI _asmaze_game_mode)))))

(event EventOnLeave
  (params (OtherActor :type Object%20Object%20Reference))
  ;[1 1 1] Call to parent
  (|CallParentFunction OtherActor)
  ;[1 1 1] Clear Tutorial Message
  (bind _isplayer (CallFunction|IsPlayer OtherActor))
  (if _isplayer
    (bind _asmaze_game_mode (Utilities|Casting|CastToMazeGameMode (Game|GetGameMode)))
    (Variables|/Game/UI/PlayerUI.PlayerUI_C|SetMessage (Variables|/Game/GameSettings/MazeGameMode.MazeGameMode_C|GetPlayerUI _asmaze_game_mode) "")
    (Default|UpdateMessage (Variables|/Game/GameSettings/MazeGameMode.MazeGameMode_C|GetPlayerUI _asmaze_game_mode))))

(event EventOnOpen
  ;[1 1 1] Call to parent
  (|CallParentFunction)
  ;[1 1 1] Clear Tutorial Message
  (bind _asmaze_game_mode (Utilities|Casting|CastToMazeGameMode (Game|GetGameMode)))
  (Variables|/Game/UI/PlayerUI.PlayerUI_C|SetMessage (Variables|/Game/GameSettings/MazeGameMode.MazeGameMode_C|GetPlayerUI _asmaze_game_mode) "")
  (Default|UpdateMessage (Variables|/Game/GameSettings/MazeGameMode.MazeGameMode_C|GetPlayerUI _asmaze_game_mode)))

(fn ConstructionScript
  (|CallParentFunction))