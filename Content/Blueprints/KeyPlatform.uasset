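; KeyPlatform is an interactable maze pickup that gives the player a key.
; Trigger volume overlaps with the player enable and disable input, so Interact only works while standing inside it.
; The first press sets a taken flag, then plays a pickup sound, destroys the key component and increments the PlayerCharacter key count.
; It then refreshes the key display through the MazeGameMode's PlayerUI.
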(event OnComponentBeginOverlap(TriggerVolume)
  (params (OverlappedComponent :type Primitive%20Component%20Object%20Reference) (OtherActor :type Actor%20Object%20Reference) (OtherComp :type Primitive%20Component%20Object%20Reference) (OtherBodyIndex :type Integer) (bFromSweep :type Boolean) (SweepResult :type Hit%20Result%20Structure%20%28by%20ref%29))
  ;[1 1 1] Bind events
  (CallFunction|OnEnter OtherActor))

(event OnComponentEndOverlap(TriggerVolume)
  (params (OverlappedComponent :type Primitive%20Component%20Object%20Reference) (OtherActor :type Actor%20Object%20Reference) (OtherComp :type Primitive%20Component%20Object%20Reference) (OtherBodyIndex :type Integer))
  ;[1 1 1] Bind events
  (CallFunction|OnLeave OtherActor))

(event Custom|OnInteract
  ;[1 1 1] Is Key not Taken?
  (if (not (Variables|Default|GetisTaken))
    (Variables|Default|SetisTaken true :!pinned true) ; Set isTaken
    (CallFunction|OnTake :!pinned true) ; Send Take Event
  ))

(event Custom|OnEnter
  (params (OtherActor :type Object%20Object%20Reference))
  (bind _isplayer (CallFunction|IsPlayer OtherActor))
  (if _isplayer
    ;[1 1 1] Enable Input
    (Input|EnableInput (Game|GetPlayerController 0))))

(event Custom|OnLeave
  (params (OtherActor :type Object%20Object%20Reference))
  (bind _isplayer (CallFunction|IsPlayer OtherActor))
  (if _isplayer
    ;[1 1 1] Disable Input
    (Input|DisableInput (Game|GetPlayerController 0))))

(event Custom|OnTake
  (bind _key (Variables|Default|GetKey))
  ;[1 1 1] Destroy Key
  (Utilities|IsValid _key
    (:Is%20Valid
      (Audio|PlaySoundatLocation "/Game/Sounds/PickupSkull_SFX.PickupSkull_SFX" (Transformation|GetActorLocation (Game|GetPlayerCharacter 0)) "0, 0, 0" 1.0 1.0 0.0 0 0 0)
      (Components|DestroyComponent _key)
      ;[1 1 1] Give Key to Player
      (bind _asplayer_character (Utilities|Casting|CastToPlayerCharacter (Game|GetPlayerCharacter 0)))
      (Math|Integer|IncrementInt (Variables|/Game/Player/PlayerCharacter.PlayerCharacter_C|GetnumberOfKeys _asplayer_character)
        (:%20%20
          ;[1 1 1] Update Number Of Keys display
          (bind _asmaze_game_mode (Utilities|Casting|CastToMazeGameMode (Game|GetGameMode)))
          (Default|UpdateNumberOfKeys (Variables|/Game/GameSettings/MazeGameMode.MazeGameMode_C|GetPlayerUI _asmaze_game_mode)))))
    (:Is%20Not%20Valid
      (Development|PrintString "Invalid Key Mesh" true true "(R=1.000000,G=0.008603,B=0.000000,A=1.000000)"))))

(event Input|ActionEvents|InputActionInteract
  (params (Key :type Key%20Structure :default "None"))
  ;[1 1 1] Bind events
  (:Pressed
    (CallFunction|OnInteract)))

(fn ConstructionScript)